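; Pickup actor that gives an overlapping Nimbus2001 the Quaffle if it has none, playing a pickup sound.
; Tick spins it by a per-frame yaw step and runs ping-pong logic between its start position and EndLocation.
; A MoveTowards helper clamps each step at the destination, but the step is Speed multiplied by zero, so as written it does not travel.
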(event `self.ReceiveBeginPlay`
  (set `self.InitialLocation` (`self.K2_GetActorLocation`))
  (set `self.TargetLocation` (`self.EndLocation`)))

(event `self.ReceiveActorBeginOverlap`
  (params (OtherActor :type "Actor Object Reference"))
  ;[1 1 1] Give Quaffle when interacted with
  (bind _asnimbus_2001 (cast `/Game/Game/Pawns/Nimbus2001` OtherActor))
  (if (not (`/Game/Game/Pawns/Nimbus2001.HasQuaffle` _asnimbus_2001))
    (set `/Game/Game/Pawns/Nimbus2001.HasQuaffle` true _asnimbus_2001)
    (`GameplayStatics.PlaySound2D` "/Game/Game/Audio/PickUp.PickUp" 1.0 1.0 0.0 null null)))

(event `self.ReceiveTick`
  (params (DeltaSeconds :type "Float (single-precision)"))
  ;[1 1 1] Rotate Object
  (`self.K2_AddActorLocalRotation` (`KismetMathLibrary.MakeRotator` 0.0 0.0 (+ (`self.RotationPerSecond`) 1.0)))
  ;[1 1 1] Move Object
  (bind _nextlocation (`self.MoveTowards` (`self.K2_GetActorLocation`) (`self.TargetLocation`) (* 0.0 (`self.Speed`))))
  (`self.K2_SetActorLocation` _nextlocation)
  (if (== (`self.TargetLocation`) (`self.K2_GetActorLocation`))
    (if (== (`self.InitialLocation`) (`self.TargetLocation`))
      (set `self.TargetLocation` (`self.EndLocation`))
      (else
        (set `self.TargetLocation` (`self.InitialLocation`))))))

(fn `MoveTowards`
  (params (CurrentLocation :type "Vector Structure") (Destination :type "Vector Structure") (MaxDeltaDistance :type "Float (double-precision)"))
  (returns (NextLocation :type "Vector Structure"))
  (bind _returnvalue (- Destination CurrentLocation))
  (bind _returnvalue_2 (* (`KismetMathLibrary.Normal` _returnvalue) MaxDeltaDistance))
  (if (< (`KismetMathLibrary.VSize` _returnvalue) (`KismetMathLibrary.VSize` _returnvalue_2))
    (return (`local.Destination`))
    (else
      (return (+ _returnvalue_2 (`local.CurrentLocation`))))))

(fn `UserConstructionScript`)