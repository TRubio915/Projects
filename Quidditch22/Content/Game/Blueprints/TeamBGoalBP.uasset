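; Team B goal actor that scores points when something other than the first player's pawn overlaps it.
; On overlap it casts the game state to Q22GameState, adds a fixed amount to TeamBPoints and plays the Goal sound at the first player controller's location.
; The overlapping actor is filtered only against that pawn, with no check for a ball or other specific class.
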(event `self.ReceiveActorBeginOverlap`
  (params (OtherActor :type "Actor Object Reference"))
  (if (not (== OtherActor (`GameplayStatics.GetPlayerPawn` 0)))
    (bind _asq22game_state (cast `/Game/Game/Blueprints/GameManagers/Q22GameState` (`GameplayStatics.GetGameState`)))
    (set `/Game/Game/Blueprints/GameManagers/Q22GameState.TeamBPoints` (+ (`/Game/Game/Blueprints/GameManagers/Q22GameState.TeamBPoints` _asq22game_state) 10) _asq22game_state)
    (`GameplayStatics.PlaySoundAtLocation` "/Game/Game/Audio/Goal.Goal" (`self.K2_GetActorLocation` (`GameplayStatics.GetPlayerController` 0)) (struct) 1.0 1.0 0.0 null null null)))

(fn `UserConstructionScript`)