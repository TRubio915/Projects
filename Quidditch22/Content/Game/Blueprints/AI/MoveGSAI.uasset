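; Behavior tree task that pushes the GSnitchAI pawn toward a location read from the Blackboard.
; A short, non-looping timer fires one acceleration force on the capsule, aimed at the target and scaled down by progress over the initial distance.
; That single tick succeeds the task if the pawn is within a small radius; the task otherwise fails after the TimeToAutofail delay.
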(event `self.ReceiveExecuteAI`
  (params (OwnerController :type "AIController Object Reference") (ControlledPawn :type "Pawn Object Reference"))
  ;[1 1 1] Setup
  (set `self.Controlled Pawn Ref` ControlledPawn)
  (set `self.MoveToLocation` (`BTFunctionLibrary.GetBlackboardValueAsVector` (`self.MoveToKey`)))
  (set `self.InitialDistance` (`self.GetDistanceToDestination`))
  ;[1 1 1] Begin Adding Force
  (bind _returnvalue (`KismetSystemLibrary.K2_SetTimerDelegate` (delegate `AddForce`) 0.01))
  (set `self.ForceTimerRef` _returnvalue)
  ;[1 1 1] Time to Autofail
  (`KismetSystemLibrary.Delay` (`self.TimeToAutofail`))
  (`self.FinishExecute` false))

(event `AddForce`
  ;[1 1 1] Add Force towards our Target Location
  (bind _asgsnitch_ai (cast `/Game/Game/Blueprints/AI/GSnitchAI` (`self.Controlled Pawn Ref`)))
  (`PrimitiveComponent.AddForce` (`Actor.GetComponentByClass` _asgsnitch_ai "/Script/Engine.CapsuleComponent") (* (`KismetMathLibrary.VLerp` (`KismetMathLibrary.GetDirectionUnitVector` (`Actor.K2_GetActorLocation` (`self.Controlled Pawn Ref`)) (`self.MoveToLocation`)) (0.0 0.0 0.0) (/ (- (`self.InitialDistance`) (`self.GetDistanceToDestination`)) (`self.InitialDistance`))) (`self.MaxForceMagnitude`)) "None" true)
  ;[1 1 1] Check if complete
  (if (<= (`self.GetDistanceToDestination`) 50.0)
    (`KismetSystemLibrary.K2_ClearAndInvalidateTimerHandle` (`self.ForceTimerRef`))
    (`KismetSystemLibrary.PrintString` "Reached Location")
    (`self.FinishExecute` true)))

(fn `GetDistanceToDestination`
  (returns (Distance :type "Float (double-precision)"))
  (return (`KismetMathLibrary.VSize` (- (`Actor.K2_GetActorLocation` (`self.Controlled Pawn Ref`)) (`self.MoveToLocation`)))))