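; Golden Snitch actor for what appears to be a Quidditch game, whose capture ends the game.
; Any actor overlap casts the game mode to Q22GameMode and calls QuitGame, without checking what overlapped.
; A separate SnitchCaught function sets IsCaught and makes the same QuitGame call, though nothing in this Blueprint calls it.
; BeginPlay prints a spawn message through the AILog helper, and no movement logic is present.
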(event `self.ReceiveBeginPlay`
  (set `self.LogMsg` "Snitch Spawned...")
  (`self.AILog`))

(event `self.ReceiveActorBeginOverlap`
  (params (OtherActor :type "Actor Object Reference"))
  (bind _asq22game_mode (cast `/Game/Game/Blueprints/Q22GameMode` (`GameplayStatics.GetGameMode`)))
  (`/Game/Game/Blueprints/Q22GameMode.Quit Game` _asq22game_mode))

(fn `AILog`
  (`KismetSystemLibrary.PrintString` (`self.LogMsg`))
  (return))

(fn `SnitchCaught`
  (set `self.isCaught` true)
  (bind _asq22game_mode (cast `/Game/Game/Blueprints/Q22GameMode` (`GameplayStatics.GetGameMode`)))
  (`/Game/Game/Blueprints/Q22GameMode.Quit Game` _asq22game_mode))

(fn `UserConstructionScript`)