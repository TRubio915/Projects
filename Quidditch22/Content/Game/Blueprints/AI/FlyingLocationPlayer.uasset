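; Behavior tree task that picks a flying move location around the player for the AI pawn.
; Random directions with halved vertical component are scaled between min and max distances from the player's position.
; A box trace from the pawn tests each point, accepting it on a hit, as the negation is unwired.
; Accepted points go to the blackboard; otherwise it retries until a never-reset counter passes its limit, then fails.
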(event `self.ReceiveExecuteAI`
  (params (OwnerController :type "AIController Object Reference") (ControlledPawn :type "Pawn Object Reference"))
  ;[1 1 1] attach
  (set `self.ControlledPawnRef` ControlledPawn)
  (set `self.ProvisionalRoamLocation` (`self.GetNewProvRoamLocation`) :!label _label)
  (bind _isvalidlocation (`self.TestProvFlyingLocation`))
  (if _isvalidlocation
    (`BTFunctionLibrary.SetBlackboardValueAsVector` (`self.MoveToLocationKey`) (`self.ProvisionalRoamLocation`))
    (`self.FinishExecute` true)
    (else
      (`/Engine/EditorBlueprintResources/StandardMacros.IncrementInt` (`self.Counter`)
        (:`  `
          (if (<= (`self.Counter`) 25)
            (goto _label)
            (else
              (`self.FinishExecute` false)
              (`KismetSystemLibrary.PrintString` "No Valid Location"))))))))

(fn `GetNewProvRoamLocation`
  (returns (NewProvRoamLoc :type "Vector Structure"))
  (locals (BallBoundsRef :type "NavMeshBoundsVolume Object Reference" :default null))
  (bind (_returnvalue_x _returnvalue_y _returnvalue_z) (`KismetMathLibrary.BreakVector` (`KismetMathLibrary.RandomUnitVector`)))
  (return (+ (* (`KismetMathLibrary.Normal` (`KismetMathLibrary.MakeVector` _returnvalue_x _returnvalue_y (/ _returnvalue_z 2.0))) (`KismetMathLibrary.RandomFloatInRange` (`self.MinDistance`) (`self.MaxDistance`))) (`Actor.K2_GetActorLocation` (`BTFunctionLibrary.GetBlackboardValueAsActor` (`self.PlayerLocation`))))))

(fn `TestProvFlyingLocation`
  (returns (isValidLocation :type Boolean))
  (bind (_outhit _returnvalue) (`KismetSystemLibrary.BoxTraceSingle` (`Actor.K2_GetActorLocation` (`self.ControlledPawnRef`)) (`self.ProvisionalRoamLocation`) (`Actor.GetActorBounds` (`self.ControlledPawnRef`) true false) (struct) "TraceTypeQuery1" false (`|MakeArray` (`self.ControlledPawnRef`) :!type "Actor Object Reference") (`self.DebugType`)))
  (return _returnvalue))