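; Golden Snitch AI pawn for a Quidditch game that ends the match when the player catches it.
; On BeginPlay it passes its behavior tree and pawn-sensing target to its MyAIC controller.
; The first player overlap, gated by DoOnce, awards Team A the catch bonus, zeroes the Nimbus2001's max speed and flags game over in Q22GameMode.
; Goal and win sounds play, then a delay returns to the main menu.
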(event `self.ReceiveBeginPlay`
  ;[1 1 1] Setup AIC for this object
  (bind _asmy_aic (cast `/Game/Game/Blueprints/AI/MyAIC` (`AIBlueprintHelperLibrary.GetAIController` self)))
  (`/Game/Game/Blueprints/AI/MyAIC.Setup AIC` _asmy_aic (`self.BT`) (`self.Player`)))

(event `self.ReceiveActorBeginOverlap`
  (params (OtherActor :type "Actor Object Reference"))
  ;[1 1 1] Win State
  (if (== OtherActor (`GameplayStatics.GetPlayerPawn` 0))
    (`/Engine/EditorBlueprintResources/StandardMacros.DoOnce` false
      (:`Completed`
        (bind _asq22game_state (cast `/Game/Game/Blueprints/GameManagers/Q22GameState` (`GameplayStatics.GetGameState`)))
        (set `/Game/Game/Blueprints/GameManagers/Q22GameState.TeamAPoints` (+ (`/Game/Game/Blueprints/GameManagers/Q22GameState.TeamAPoints` _asq22game_state) 150) _asq22game_state)
        (bind _asnimbus_2001 (cast `/Game/Game/Pawns/Nimbus2001` (`GameplayStatics.GetPlayerPawn` 0)))
        (set `/Game/Game/Pawns/Nimbus2001.MaxSpeed` 0.0 _asnimbus_2001)
        (`GameplayStatics.PlaySoundAtLocation` "/Game/Game/Audio/Goal.Goal" (`self.K2_GetActorLocation` (`GameplayStatics.GetPlayerController` 0)) (struct) 1.0 1.0 0.0 null null null)
        (bind _asq22game_mode (cast `/Game/Game/Blueprints/GameManagers/Q22GameMode` (`GameplayStatics.GetGameMode`)))
        (set `/Game/Game/Blueprints/GameManagers/Q22GameMode.GameOver` true _asq22game_mode)
        (`GameplayStatics.PlaySound2D` "/Game/Game/Audio/Win.Win" 1.0 1.0 0.0 null null)
        (`KismetSystemLibrary.Delay` 7.5)
        (`GameplayStatics.OpenLevel` "MainMenuLevel")))))

(fn `UserConstructionScript`)