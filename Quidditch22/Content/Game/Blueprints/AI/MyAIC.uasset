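; AI controller that runs a supplied behavior tree and reports pawn-sensing sightings of one target to its blackboard.
; SetupAIC starts the tree and stores the target and the controlled pawn's starting location as Origin.
; Seeing the target sets CanSeeTarget and SeenRecently, with retriggerable delays scaled to the sensing interval acting as sight timeouts.
; Both timeouts clear CanSeeTarget, so SeenRecently is never reset here.
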(event `self.ReceiveBeginPlay`)

(event `Setup AIC`
  (params (BT :type "BehaviorTree Object Reference") (PawnSensingTarget :type "/Game/Game/Pawns/Nimbus2001 Object Reference"))
  ;[1 1 1] Setup AI Controller
  (set `self.BT` BT)
  (set `self.PawnSensingTarget` PawnSensingTarget)
  (`self.RunBehaviorTree` (`self.BT`))
  (`/Game/Game/Blueprints/AI/AIFunctions.Update BBKey` self "Target" "NewEnumerator1" true (`self.PawnSensingTarget`))
  (`/Game/Game/Blueprints/AI/AIFunctions.Update BBKey` self "Origin" "NewEnumerator2" true null (`self.K2_GetActorLocation` (`self.K2_GetPawn`))))

(event `self.PawnSensing.OnSeePawn`
  (params (Pawn :type "Pawn Object Reference"))
  ;[1 1 1] Seeing Player Target
  (if (== Pawn (`self.PawnSensingTarget`))
    (`|ExecutionSequence`
      (:`then_0`
        (`/Game/Game/Blueprints/AI/AIFunctions.Update BBKey` self "CanSeeTarget" "NewEnumerator0" true)
        (`KismetSystemLibrary.PrintString` "Can See")
        (`KismetSystemLibrary.RetriggerableDelay` (* (`PawnSensingComponent.SensingInterval` (`self.PawnSensing`)) 2.0))
        (`/Game/Game/Blueprints/AI/AIFunctions.Update BBKey` self "CanSeeTarget"))
      (:`then_1`
        (`/Game/Game/Blueprints/AI/AIFunctions.Update BBKey` self "SeenRecently" "NewEnumerator0" true)
        (`KismetSystemLibrary.PrintString` "Can't See")
        (`KismetSystemLibrary.RetriggerableDelay` (* (`PawnSensingComponent.SensingInterval` (`self.PawnSensing`)) 5.0))
        (`/Game/Game/Blueprints/AI/AIFunctions.Update BBKey` self "CanSeeTarget")))))

(fn `UserConstructionScript`)