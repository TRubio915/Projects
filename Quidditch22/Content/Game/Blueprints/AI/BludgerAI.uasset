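; Bludger enemy AI that damages the player's Nimbus2001 broom pawn on contact.
; On BeginPlay it passes its behavior tree and player sensing target to its MyAIC controller.
; When it hits player 0's pawn, it reduces that pawn's HP by a fixed amount and plays a hit sound at the player controller's location.
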(event `self.ReceiveHit`
  (params (MyComp :type "PrimitiveComponent Object Reference") (Other :type "Actor Object Reference") (OtherComp :type "PrimitiveComponent Object Reference") (bSelfMoved :type Boolean) (HitLocation :type "Vector Structure") (HitNormal :type "Vector Structure") (NormalImpulse :type "Vector Structure") (Hit :type "HitResult Structure (by ref)"))
  (bind _returnvalue (`GameplayStatics.GetPlayerPawn` 0))
  ;[1 1 1] Damge Player
  (if (== Other _returnvalue)
    (bind _asnimbus_2001 (cast `/Game/Game/Pawns/Nimbus2001` _returnvalue))
    (`/Game/Game/Pawns/Nimbus2001.AdjustHP` _asnimbus_2001 -5.0)
    (`GameplayStatics.PlaySoundAtLocation` "/Game/Game/Audio/HitByB.HitByB" (`self.K2_GetActorLocation` (`GameplayStatics.GetPlayerController` 0)) (struct) 1.0 1.0 0.0 null null null)))

(event `self.ReceiveBeginPlay`
  ;[1 1 1] Setup AIC for this object
  (bind _asmy_aic (cast `/Game/Game/Blueprints/AI/MyAIC` (`AIBlueprintHelperLibrary.GetAIController` self)))
  (`/Game/Game/Blueprints/AI/MyAIC.Setup AIC` _asmy_aic (`self.BT`) (`self.Player`)))

(fn `UserConstructionScript`)