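; Game mode for Q22 that starts the match audio and player HUD and handles player spawn, goal scoring and quitting.
; BeginPlay plays music and crowd sound, creates the PlayerUI widget, then disables on-screen debug messages.
; Spawn, goal and quit functions write to Q22GameState, with goal points always added to Team A.
; Each event stores its message in the game state's LogMsg and prints it through GamePlayLog.
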(event `self.ReceiveBeginPlay`
  (`GameplayStatics.PlaySound2D` "/Game/Game/Audio/BkgMusic2.BkgMusic2" 1.0 1.0 0.0 null null)
  (`GameplayStatics.PlaySoundAtLocation` "/Game/Game/Audio/Crowd.Crowd" (0.0 0.0 5000.0) (struct) 1.0 1.0 0.0 null null null)
  (bind _asq22game_state (cast `/Game/Game/Blueprints/GameManagers/Q22GameState` (`GameplayStatics.GetGameState`)))
  (set `/Game/Game/Blueprints/GameManagers/Q22GameState.LogMsg` "Game Starting..." _asq22game_state)
  (bind _logmsg (`self.Game Play Log`))
  (`KismetSystemLibrary.PrintString` _logmsg)
  (bind _returnvalue (`|CreateWidget` "/Game/Game/UI/PlayerUI.PlayerUI_C" (`GameplayStatics.GetPlayerController` 0)))
  (bind _output_get (set `self.PlayerUI` _returnvalue))
  (`UserWidget.AddToViewport` _returnvalue 0)
  (`KismetSystemLibrary.ExecuteConsoleCommand` "DisableAllScreenMessages" null))

(fn `Game Play Log`
  (returns (LogMsg :type String))
  (bind _asq22game_state (cast `/Game/Game/Blueprints/GameManagers/Q22GameState` (`GameplayStatics.GetGameState`)))
  (return (`/Game/Game/Blueprints/GameManagers/Q22GameState.LogMsg` _asq22game_state)))

(fn `GoalMade`
  (params (Points :type Integer))
  (bind _asq22game_state (cast `/Game/Game/Blueprints/GameManagers/Q22GameState` (`GameplayStatics.GetGameState`)))
  (set `/Game/Game/Blueprints/GameManagers/Q22GameState.TeamAPoints` (+ Points (`/Game/Game/Blueprints/GameManagers/Q22GameState.TeamAPoints` _asq22game_state)) _asq22game_state)
  (set `/Game/Game/Blueprints/GameManagers/Q22GameState.LogMsg` "Goal Made!" _asq22game_state)
  (bind _logmsg (`self.Game Play Log`))
  (`KismetSystemLibrary.PrintString` _logmsg))

(fn `PlayerSpawn`
  (bind _asq22game_state (cast `/Game/Game/Blueprints/GameManagers/Q22GameState` (`GameplayStatics.GetGameState`)))
  (set `/Game/Game/Blueprints/GameManagers/Q22GameState.PlayerAlive` true _asq22game_state)
  (set `/Game/Game/Blueprints/GameManagers/Q22GameState.LogMsg` "Player Spawned" _asq22game_state)
  (bind _logmsg (`self.Game Play Log`))
  (`KismetSystemLibrary.PrintString` _logmsg))

(fn `Quit Game`
  (bind _asq22game_state (cast `/Game/Game/Blueprints/GameManagers/Q22GameState` (`GameplayStatics.GetGameState`)))
  (set `/Game/Game/Blueprints/GameManagers/Q22GameState.LogMsg` "Game Ending..." _asq22game_state)
  (bind _logmsg (`self.Game Play Log`))
  (`KismetSystemLibrary.PrintString` _logmsg)
  (`KismetSystemLibrary.QuitGame` null "Quit"))

(fn `UserConstructionScript`)